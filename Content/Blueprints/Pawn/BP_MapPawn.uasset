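; BP_MapPawn is a pawn that tracks the actor it overlaps and responds to a select input.
; Begin overlap stores the other actor, and any end overlap clears the reference, so only one actor is tracked at a time.
; IA_Select currently only prints a debug string when that reference is valid.
; IsOverlapping and GetOverlappedActor expose the overlap state to other code.
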(event `self.ReceiveActorBeginOverlap`
  (params (OtherActor :type "Actor Object Reference"))
  (set `self.OverlappedActor` OtherActor))

(event `self.ReceiveActorEndOverlap`
  (params (OtherActor :type "Actor Object Reference"))
  (set `self.OverlappedActor` null))

(event `EnhancedInput|/Game/Inputs/IA_Select`
  (params (ActionValue :type Boolean) (ElapsedSeconds :type "Float (double-precision)") (TriggeredSeconds :type "Float (double-precision)") (InputAction :type "InputAction Object Reference" :default "/Game/Inputs/IA_Select.IA_Select"))
  (:`Triggered`
    (`self.OverlappedActor`
      (:`then`
        (`KismetSystemLibrary.PrintString` "Pawn"))
      (:`else`))))

(fn `GetOverlappedActor`
  (returns (OverlappedActor :type "Actor Object Reference"))
  (return (`self.OverlappedActor`)))

(fn `IsOverlapping`
  (returns (IsOverlapping :type Boolean))
  (return (`KismetSystemLibrary.IsValid` (`self.OverlappedActor`))))

(fn `UserConstructionScript`)