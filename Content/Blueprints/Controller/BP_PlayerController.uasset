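; Player controller that sets up the layered game UI and turns Enhanced Input into pawn movement, camera look and game menu access.
; On BeginPlay it adds the mapping context, then activates the root layout and pushes the main game widget through CLGameInstanceSubsystem.
; Movement follows control rotation, with forward input including pitch, and look drives yaw and pitch.
; The menu action pushes GameMenuWidget, if valid, to the GameMenu layer and pauses the game.
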(event `self.ReceiveBeginPlay`
  (bind _returnvalue (subsystem `CLGameInstanceSubsystem`))
  (`self.SetInputContext`)
  (`CLGameInstanceSubsystem.ActivateLayout` _returnvalue "/Game/UI/WBP_Root.WBP_Root_C")
  (`CLGameInstanceSubsystem.PushToLayer` _returnvalue "/Game/UI/Game/WBP_GameLayerMain.WBP_GameLayerMain_C" (struct :`TagName` "Layout.Layer.Game")))

(event `SetInputContext`
  (`EnhancedInputSubsystemInterface.AddMappingContext` (subsystem `EnhancedInputLocalPlayerSubsystem`) (`self.Mapping Context`) 0 (struct)))

(event `EnhancedInput|/Game/Inputs/IA_Move`
  (params (ActionValue :type "Vector2D Structure") (ElapsedSeconds :type "Float (double-precision)") (TriggeredSeconds :type "Float (double-precision)") (InputAction :type "InputAction Object Reference" :default "/Game/Inputs/IA_Move.IA_Move"))
  (:`Triggered`
    (`self.MoveAction` ActionValue_X ActionValue_Y)))

(event `EnhancedInput|/Game/Inputs/IA_Look`
  (params (ActionValue :type "Vector2D Structure") (ElapsedSeconds :type "Float (double-precision)") (TriggeredSeconds :type "Float (double-precision)") (InputAction :type "InputAction Object Reference" :default "/Game/Inputs/IA_Look.IA_Look"))
  (:`Triggered`
    (`self.LookAction` ActionValue_X ActionValue_Y)))

(event `EnhancedInput|/Game/Inputs/IA_GameMenu`
  (params (ActionValue :type Boolean) (ElapsedSeconds :type "Float (double-precision)") (TriggeredSeconds :type "Float (double-precision)") (InputAction :type "InputAction Object Reference" :default "/Game/Inputs/IA_GameMenu.IA_GameMenu"))
  (bind _gamemenuwidget (`self.GameMenuWidget`))
  (:`Triggered`
    (if (`KismetSystemLibrary.IsValidClass` _gamemenuwidget)
      (`CLGameInstanceSubsystem.PushToLayer` (subsystem `CLGameInstanceSubsystem`) _gamemenuwidget (struct :`TagName` "Layout.Layer.GameMenu"))
      (`GameplayStatics.SetGamePaused` true))))

(fn `LookAction`
  (params (ValueX :type "Float (double-precision)") (ValueY :type "Float (double-precision)"))
  (bind _returnvalue (`self.K2_GetPawn`))
  (`Pawn.AddControllerYawInput` _returnvalue ValueX)
  (`Pawn.AddControllerPitchInput` _returnvalue ValueY))

(fn `MoveAction`
  (params (ValueX :type "Float (double-precision)") (ValueY :type "Float (double-precision)"))
  (bind (_returnvalue_roll _returnvalue_pitch _returnvalue_yaw) (`KismetMathLibrary.BreakRotator` (`self.GetControlRotation`)))
  (bind (_returnvalue_roll_2 _returnvalue_pitch_2 _returnvalue_yaw_2) (`KismetMathLibrary.BreakRotator` (`self.GetControlRotation`)))
  (`|ExecutionSequence`
    (:`then_0`
      (`Pawn.AddMovementInput` (`self.K2_GetPawn`) (`KismetMathLibrary.GetRightVector` (`KismetMathLibrary.MakeRotator` _returnvalue_roll_2 0.0 _returnvalue_yaw_2)) ValueX false))
    (:`then_1`
      (`Pawn.AddMovementInput` (`self.K2_GetPawn`) (`KismetMathLibrary.GetForwardVector` (`KismetMathLibrary.MakeRotator` 0.0 _returnvalue_pitch _returnvalue_yaw)) ValueY false))))

(fn `UserConstructionScript`)